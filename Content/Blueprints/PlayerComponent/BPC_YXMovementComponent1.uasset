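; Player component on the VR pawn that turns arm swinging into a boost from walking toward running speed.
; Each tick, when both motion controller grips' vertical velocities reach a swing threshold, their magnitudes are added to the current speed, doubled and clamped between walking and running speed.
; In walking mode, speed above walking pace decays linearly over time and is pushed to the pawn through ChangeSpeed.
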(event `self.ReceiveBeginPlay`
  (bind _asvrpawn (cast `/Game/Blueprints/VRPawn` (`self.GetOwner`)))
  (bind _output_get (set `self.Player` _asvrpawn))
  (set `self.WalkingSpeed` (`/Game/Blueprints/VRPawn.WalkingSpeed` _output_get)))

(event `self.ReceiveTick`
  (params (DeltaSeconds :type "Float (single-precision)"))
  (bind _player (`self.Player`))
  (bind _swingboundary (`self.SwingBoundary`))
  (bind _returnvalue (`KismetMathLibrary.Abs` (.z (`MotionControllerComponent.GetLinearVelocity` (`/Game/Blueprints/VRPawn.MotionControllerRightGrip` _player)))))
  (bind _returnvalue_2 (`KismetMathLibrary.Abs` (.z (`MotionControllerComponent.GetLinearVelocity` (`/Game/Blueprints/VRPawn.MotionControllerLeftGrip` _player)))))
  (`|ExecutionSequence`
    (:`then_0`
      (if (`/Game/Blueprints/VRPawn.IsInWalkingMode` (`self.Player`))
        (if (> (`self.Speed`) (`self.WalkingSpeed`))
          (set `self.Speed` (- (`self.Speed`) (* DeltaSeconds 1000.0)))
          (`/Game/Blueprints/VRPawn.ChangeSpeed` (`self.Player`) (`self.Speed`)))))
    (:`then_1`
      (if (and (>= _returnvalue_2 _swingboundary) (>= _returnvalue _swingboundary))
        (set `self.Speed` (`KismetMathLibrary.FClamp` (* (+ _returnvalue_2 _returnvalue (`self.Speed`)) 2.0) (`self.WalkingSpeed`) (`self.RunningSpeed`)))))))