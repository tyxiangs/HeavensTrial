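; VR player component that makes the VRPawn slide forward when the player crouches, detected by a low camera height.
; Each tick while crouched, a downward trace measures ground slope; steep ground sustains the slide at SlidingSpeed along the capsule's forward vector.
; On flatter ground the push lasts about a second until a delayed stop flag, which standing up resets.
; Outside walking mode, Speed decays over time and is passed to the pawn.
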(event `self.ReceiveBeginPlay`
  (bind _asvrpawn (cast `/Game/Blueprints/VRPawn` (`self.GetOwner`)))
  (set `self.Player` _asvrpawn))

(event `self.ReceiveTick`
  (params (DeltaSeconds :type "Float (single-precision)"))
  (bind _player (`self.Player`))
  (bind _player_2 (`self.Player`))
  (bind _returnvalue (`Actor.K2_GetActorLocation` (`self.Player`)))
  (bind (_relativelocation_x _relativelocation_y _relativelocation_z) (`KismetMathLibrary.BreakVector` (`SceneComponent.RelativeLocation` (`/Game/Blueprints/VRPawn.Camera` (`self.Player`)))))
  (`|ExecutionSequence`
    (:`then_0`
      (if (`/Game/Blueprints/VRPawn.IsInWalkingMode` (`self.Player`))
        _
        (elif (>= (`self.Speed`) 0.0)
          (set `self.Speed` (- (`self.Speed`) (* DeltaSeconds 1000.0)))
          (`/Game/Blueprints/VRPawn.ChangeSpeed` (`self.Player`) (`self.Speed`)))))
    (:`then_1`
      (if (< _relativelocation_z 105.0)
        (bind _outhit (`KismetSystemLibrary.LineTraceSingle` _returnvalue (+ _returnvalue (0.0 0.0 -10000.0)) "TraceTypeQuery1"))
        (if (> (`KismetMathLibrary.DegAcos` (`KismetMathLibrary.Dot_VectorVector` (0.0 0.0 1.0) (`.ImpactNormal` (`GameplayStatics.BreakHitResult` _outhit)))) 15.0)
          (set `self.IsSliding` true)
          (set `self.IsStopTrigger` false)
          (set `self.Speed` (`self.SlidingSpeed`))
          (`Pawn.AddMovementInput` _player_2 (`SceneComponent.GetForwardVector` (`Character.CapsuleComponent` _player_2)) 1.0 false)
          (elif (not (`self.IsStopTrigger`))
            (set `self.Speed` (`self.SlidingSpeed`))
            (`Pawn.AddMovementInput` _player (`SceneComponent.GetForwardVector` (`Character.CapsuleComponent` _player)) 1.0 false)
            (if (`self.IsSliding`)
              (set `self.IsSliding` false)
              (elif (not (`self.IsStopTrigger`))
                (`KismetSystemLibrary.Delay` 1.0)
                (set `self.IsStopTrigger` true)))))
        (else
          (set `self.IsSliding` false)
          (set `self.IsStopTrigger` false))))))