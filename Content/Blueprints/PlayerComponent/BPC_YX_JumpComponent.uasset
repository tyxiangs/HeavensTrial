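; Actor component for the VR pawn that turns an upward swing of both hands into a character jump.
; YXJump runs only while the pawn is in jumping mode and no earlier check is pending, using IsJumpingFinished as a re-entry guard.
; It samples both grip controllers' world positions across a very short delay and calls Jump when both rise past a fixed height threshold.
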(event `YXJump`
  (bind _player (`self.Player`))
  (bind (_leftdifference_x _leftdifference_y _leftdifference_z) (`KismetMathLibrary.BreakVector` (`self.LeftDifference`)))
  (bind (_rightdifference_x _rightdifference_y _rightdifference_z) (`KismetMathLibrary.BreakVector` (`self.RightDifference`)))
  (bind _player_2 (`self.Player`))
  (bind _player_3 (`self.Player`))
  (bind _player_4 (`self.Player`))
  (bind _asvrpawn (cast `/Game/Blueprints/VRPawn` (`self.GetOwner`)))
  (set `self.Player` _asvrpawn)
  (if (`/Game/Blueprints/VRPawn.IsJumpingMode` _player)
    (if (`/Game/Blueprints/VRPawn.IsJumpingFinished` _player)
      (if true
        (set `/Game/Blueprints/VRPawn.IsJumpingFinished` false _player_4)
        (set `self.PrevRightHandPos` (`SceneComponent.K2_GetComponentLocation` (`/Game/Blueprints/VRPawn.MotionControllerRightGrip` _player_4)))
        (set `self.PrevLeftHandPos` (`SceneComponent.K2_GetComponentLocation` (`/Game/Blueprints/VRPawn.MotionControllerLeftGrip` _player_4)))
        (`KismetSystemLibrary.Delay` 0.01)
        (set `self.RightDifference` (- (`SceneComponent.K2_GetComponentLocation` (`/Game/Blueprints/VRPawn.MotionControllerRightGrip` _player_3)) (`self.PrevRightHandPos`)))
        (set `self.LeftDifference` (- (`SceneComponent.K2_GetComponentLocation` (`/Game/Blueprints/VRPawn.MotionControllerLeftGrip` _player_3)) (`self.PrevLeftHandPos`)))
        (if (and (>= _leftdifference_z 1.5) (>= _rightdifference_z 1.5))
          (cast `Character` (`self.GetOwner`))
          (`Character.Jump` _player_2))
        (set `/Game/Blueprints/VRPawn.IsJumpingFinished` true _player_2)))))