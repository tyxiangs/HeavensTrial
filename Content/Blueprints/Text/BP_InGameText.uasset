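; BP_InGameText is an in-world text actor that shows a message when the VR player comes near and turns to face them.
; A capsule overlap with a VRPawn stores the pawn and reveals the TextRender and Niagara component, and leaving clears the reference and hides both.
; While a pawn is stored, Tick rotates the whole actor toward it with a look-at rotation.
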(event `self.ReceiveBeginPlay`
  (`self.SetTextVisibility` false)
  (`TextRenderComponent.K2_SetText` (`self.TextRender`) (`self.Text`)))

(event `self.ReceiveTick`
  (params (DeltaSeconds :type "Float (single-precision)"))
  (bind _playerref (`self.PlayerRef`))
  (`/Engine/EditorBlueprintResources/StandardMacros.IsValid` _playerref
    (:`Is Valid`
      (`self.K2_SetActorRotation` (`KismetMathLibrary.FindLookAtRotation` (`self.K2_GetActorLocation`) (`self.K2_GetActorLocation` _playerref))))))

(event `self.Capsule.OnComponentBeginOverlap`
  (params (OverlappedComponent :type "PrimitiveComponent Object Reference") (OtherActor :type "Actor Object Reference") (OtherComp :type "PrimitiveComponent Object Reference") (OtherBodyIndex :type Integer) (bFromSweep :type Boolean) (SweepResult :type "HitResult Structure (by ref)"))
  (bind _asvrpawn (cast `/Game/Blueprints/VRPawn` OtherActor))
  (set `self.PlayerRef` _asvrpawn)
  (`self.SetTextVisibility` true))

(event `self.Capsule.OnComponentEndOverlap`
  (params (OverlappedComponent :type "PrimitiveComponent Object Reference") (OtherActor :type "Actor Object Reference") (OtherComp :type "PrimitiveComponent Object Reference") (OtherBodyIndex :type Integer))
  (cast `/Game/Blueprints/VRPawn` OtherActor)
  (set `self.PlayerRef` null)
  (`self.SetTextVisibility` false))

(fn `SetTextVisibility`
  (params (isVisible :type Boolean))
  (`SceneComponent.SetVisibility` (`self.Niagara`) isVisible true)
  (`SceneComponent.SetVisibility` (`self.TextRender`) isVisible false))

(fn `UserConstructionScript`)