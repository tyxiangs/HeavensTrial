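; VR pawn component that triggers a physical-gesture jump when both motion controllers move upward quickly.
; YXJump samples both grip world positions across a very short Delay and calls Jump if both rose past a Z threshold.
; The pawn's IsJumpingFinished flag blocks re-entry during sampling and resets right after the check.
; Jump, land and grunt audio setup and playback nodes are present but disconnected.
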(event `self.ReceiveBeginPlay`
  (bind _asvrpawn (cast `/Game/Blueprints/VRPawn` (`self.GetOwner`)))
  (set `self.Player` _asvrpawn))

(event `YXJump`
  (bind (_rightdifference_x _rightdifference_y _rightdifference_z) (`KismetMathLibrary.BreakVector` (`self.RightDifference`)))
  (bind (_leftdifference_x _leftdifference_y _leftdifference_z) (`KismetMathLibrary.BreakVector` (`self.LeftDifference`)))
  (bind _player (`self.Player`))
  (bind _player_2 (`self.Player`))
  (bind _player_3 (`self.Player`))
  (if (`/Game/Blueprints/VRPawn.IsJumpingFinished` (`self.Player`))
    (`KismetSystemLibrary.PrintString` "Jump Pressed")
    (set `/Game/Blueprints/VRPawn.IsJumpingFinished` false _player_3)
    (set `self.PrevRightHandPos` (`SceneComponent.K2_GetComponentLocation` (`/Game/Blueprints/VRPawn.MotionControllerRightGrip` _player_3)))
    (set `self.PrevLeftHandPos` (`SceneComponent.K2_GetComponentLocation` (`/Game/Blueprints/VRPawn.MotionControllerLeftGrip` _player_3)))
    (`KismetSystemLibrary.Delay` 0.01)
    (set `self.RightDifference` (- (`SceneComponent.K2_GetComponentLocation` (`/Game/Blueprints/VRPawn.MotionControllerRightGrip` _player_2)) (`self.PrevRightHandPos`)))
    (set `self.LeftDifference` (- (`SceneComponent.K2_GetComponentLocation` (`/Game/Blueprints/VRPawn.MotionControllerLeftGrip` _player_2)) (`self.PrevLeftHandPos`)))
    (if (and (>= _leftdifference_z 1.5) (>= _rightdifference_z 1.5))
      (cast `Character` (`self.GetOwner`))
      (`Character.Jump` _player))
    (set `/Game/Blueprints/VRPawn.IsJumpingFinished` true _player)))