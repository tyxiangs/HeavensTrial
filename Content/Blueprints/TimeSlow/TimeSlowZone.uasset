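; TimeSlowZone is an actor that slows the whole game through global time dilation while fading a post-process colour effect.
; After a short delay on BeginPlay, it plays a clock-ticking cue and runs a timeline that drives a dynamic material's BW_Amount and reapplies the slow factor each update.
; Its Destroyer event stops the sound, destroys the actor and restores normal time; overlap detection is unused.
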(event `self.ReceiveBeginPlay`
  (`KismetSystemLibrary.Delay` 0.2)
  (bind _returnvalue (`KismetMaterialLibrary.CreateDynamicMaterialInstance` "/Game/Blueprints/TimeSlow/PostProcessMaterial.PostProcessMaterial"))
  (set `self.DynamicPPMaterial` _returnvalue)
  (`AudioComponent.Play` (`self.11L-clock_ticking-49566274_Cue`) 0.0)
  (bind (_direction _bwtonormal) (`Timeline|ColourChange` :!via `PlayFromStart`)
    (:`Update`
      (`PostProcessComponent.AddOrUpdateBlendable` (`self.PostProcess`) (`self.DynamicPPMaterial`) 1.0)
      (`MaterialInstanceDynamic.SetScalarParameterValue` (`self.DynamicPPMaterial`) "BW_Amount" _bwtonormal)
      (`self.Slow Time`))))

(event `Destroyer`
  (`AudioComponent.Stop` (`self.11L-clock_ticking-49566274_Cue`))
  (`self.K2_DestroyActor`)
  (`self.Resume Time`))

(fn `Resume Time`
  (`GameplayStatics.SetGlobalTimeDilation` 1.0))

(fn `Slow Time`
  (`GameplayStatics.SetGlobalTimeDilation` (`self.SlowFactor`)))

(fn `UserConstructionScript`)