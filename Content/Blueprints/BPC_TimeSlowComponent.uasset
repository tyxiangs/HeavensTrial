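; Actor component for the VR pawn that lets the player place a time-slow zone.
; Start plays a whoosh and, if charge remains, spawns a TimeSlowZone ahead of the camera at eye height; End destroys it with a reverse whoosh.
; Charge drain, regeneration and auto-end logic is disconnected from Tick, so never runs.
; Global time-dilation helper functions exist but are not called here.
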(event `self.ReceiveTick`
  (params (DeltaSeconds :type "Float (single-precision)")))

(event `self.ReceiveBeginPlay`
  (bind _asvrpawn (cast `/Game/Blueprints/VRPawn` (`self.GetOwner`)))
  (set `self.Player` _asvrpawn))

(event `TimeSlowStart`
  (bind _camera (`/Game/Blueprints/VRPawn.Camera` (`self.Player`)))
  (bind (_returnvalue_x _returnvalue_y _returnvalue_z) (`KismetMathLibrary.BreakVector` (`SceneComponent.K2_GetComponentLocation` _camera)))
  (bind (_returnvalue_x_2 _returnvalue_y_2) (`KismetMathLibrary.BreakVector` (+ (* (`SceneComponent.GetForwardVector` _camera) 400.0) (`SceneComponent.K2_GetComponentLocation` _camera))))
  (if (not (`self.IsTriggered`))
    (set `self.IsTriggered` true)
    (if (> (`self.TimeSlowProgress`) 0.0)
      (`GameplayStatics.SpawnSoundAtLocation` "/Game/Blueprints/YX_SoundEffect/whoosh-fast-bright-vadi-sound-1-00-01.whoosh-fast-bright-vadi-sound-1-00-01" (`SceneComponent.K2_GetComponentLocation` (`Character.CapsuleComponent` (`self.Player`))) (struct) 1.0 1.0 0.0 null null)
      (bind _returnvalue (`|SpawnActorFromClass` "/Game/Blueprints/TimeSlow/TimeSlowZone.TimeSlowZone_C" (`KismetMathLibrary.Conv_VectorToTransform` (`KismetMathLibrary.MakeVector` _returnvalue_x_2 _returnvalue_y_2 _returnvalue_z)) "Undefined" "MultiplyWithRoot" null null))
      (set `self.Zone` _returnvalue))))

(event `TimeSlowEnd`
  (`/Engine/EditorBlueprintResources/StandardMacros.IsValid` (`self.Zone`)
    (:`Is Valid`
      (set `self.IsTriggered` false)
      (`GameplayStatics.SpawnSoundAtLocation` "/Game/Blueprints/YX_SoundEffect/SW_ReverseWhoosh_Cue.SW_ReverseWhoosh_Cue" (`SceneComponent.K2_GetComponentLocation` (`Character.CapsuleComponent` (`self.Player`))) (struct) 1.0 1.0 0.0 null null)
      (`/Game/Blueprints/TimeSlow/TimeSlowZone.Destroyer` (`self.Zone`)))))

(fn `ResumeTime`
  (`GameplayStatics.SetGlobalTimeDilation` 1.0))

(fn `SlowTime`
  (`GameplayStatics.SetGlobalTimeDilation` (`self.SlowFactor`)))