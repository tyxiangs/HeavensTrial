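; Base enemy projectile that flies at a set speed toward a Target and reports hits on it.
; Construction applies Speed to the movement component, and BeginPlay aims velocity once at a point above the target's capsule, without homing.
; A box hit on the Target calls OnProjectileHit with its damage component and DamageInfo, and any hit destroys the projectile.
; The owner ignore call passes false, so it does not enable ignoring the owner.
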(event `self.ReceiveBeginPlay`
  ; Initialize direction of projectile and ignore collision with enemy class
  (`self.Target`
    (:`then`
      (`self.RotateToTarget`)
      (`PrimitiveComponent.IgnoreActorWhenMoving` (`self.Box`) (`self.GetOwner`) false))
    (:`else`)))

(event `self.Box.OnComponentHit`
  (params (HitComponent :type "PrimitiveComponent Object Reference") (OtherActor :type "Actor Object Reference") (OtherComp :type "PrimitiveComponent Object Reference") (NormalImpulse :type "Vector Structure") (Hit :type "HitResult Structure (by ref)"))
  (bind _returnvalue (`self.GetComponentByClass` OtherActor "/Game/DamageSystem/BPC_LX_DamageComponent.BPC_LX_DamageComponent_C"))
  (if (== OtherActor (`self.Target`))
    (`KismetSystemLibrary.PrintString` "Projectile hit target!")
    (if (`KismetSystemLibrary.IsValid` _returnvalue)
      (`self.OnProjectileHit` _returnvalue (`self.DamageInfo`) Hit))
    (`self.K2_DestroyActor`)
    (else
      (`self.K2_DestroyActor`))))

(fn `RotateToTarget`
  (set `MovementComponent.Velocity` (* (`KismetMathLibrary.GetDirectionUnitVector` (`self.K2_GetActorLocation`) (+ (`SceneComponent.K2_GetComponentLocation` (`self.GetComponentByClass` (`self.Target`) "/Script/Engine.CapsuleComponent")) (0.0 0.0 50.0))) (`self.Speed`)) (`self.ProjectileMovement`)))

(fn `UserConstructionScript`
  (bind _projectilemovement (`self.ProjectileMovement`))
  (set `ProjectileMovementComponent.InitialSpeed` (`self.Speed`) _projectilemovement)
  (set `ProjectileMovementComponent.MaxSpeed` (`self.Speed`) _projectilemovement))