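; BP_LX_LightBall is an enemy light ball that the player can apparently parry by slashing it.
; Slash calls Parried, which replaces the ball with a BP_LX_ParriedLightBall at the same transform, passing on its Speed and targeting the original owner.
; The parry also prints the owner's name, spawns a wind VFX, plays a slice sound and destroys the ball.
; The graph itself contains no movement or hit logic.
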(event `/Game/BlueprintInterface/BPI_Slashable.Slash`
  (params (Impulse :type "Vector Structure"))
  (`self.Parried`))

(event `Parried`
  (bind _returnvalue (`self.GetOwner`))
  (`KismetSystemLibrary.PrintString` (`KismetSystemLibrary.GetDisplayName` _returnvalue))
  (`|SpawnActorFromClass` "/Game/Blueprints/Enemy/BP_LX_ParriedLightBall.BP_LX_ParriedLightBall_C" (`self.GetTransform`) "AdjustIfPossibleButAlwaysSpawn" "MultiplyWithRoot" _returnvalue (`self.Speed`) _returnvalue null)
  (`|SpawnActorFromClass` "/Game/Blueprints/Enemy/BP_ParriedVFX_Wind.BP_ParriedVFX_Wind_C" (`KismetMathLibrary.MakeTransform` (`self.K2_GetActorLocation`) (struct) (0.5 0.5 0.5)) "AlwaysSpawn" "MultiplyWithRoot" null null)
  (`GameplayStatics.PlaySoundAtLocation` "/Game/Blueprints/Sword/slice.slice" (`self.K2_GetActorLocation`) (struct) 1.0 1.0 0.0 null null null null)
  (`self.K2_DestroyActor`))

(fn `UserConstructionScript`
  (`parent.UserConstructionScript`))