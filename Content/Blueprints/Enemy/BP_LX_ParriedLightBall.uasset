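; BP_LX_ParriedLightBall is an enemy light-ball projectile variant, named as the parried version, that deals half its configured damage.
; Its construction script runs the parent's, binds an event to OnProjectileHit and rebuilds DamageInfo with the amount halved, keeping type and response.
; The DamageTarget event applies that damage struct to the other actor and spawns blood particles and a grunt sound at the projectile's location.
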(event `DamageTarget`
  (params (OtherActor :type "/Game/DamageSystem/BPC_LX_DamageComponent Object Reference") (DamageInfo :type "/Game/DamageSystem/S_LX_DamageInfo Structure") (Hit :type "HitResult Structure"))
  (`/Game/DamageSystem/BPI_LX_Damagable.TakeDamage` OtherActor DamageInfo)
  (`GameplayStatics.SpawnEmitterAtLocation` "/Game/Blueprints/Sword/P_Blood.P_Blood" (`self.K2_GetActorLocation`))
  (`GameplayStatics.PlaySoundAtLocation` "/Game/Blueprints/Enemy/SW_AttackedGrunt.SW_AttackedGrunt" (`self.K2_GetActorLocation`) (struct) 1.0 1.0 0.0 null null null null))

(fn `UserConstructionScript`
  (bind (_amount _damagetype _damageresponse) (break `/Game/DamageSystem/S_LX_DamageInfo` (`self.DamageInfo`)))
  (`parent.UserConstructionScript`)
  (add `self.OnProjectileHit` (`|CreateDelegate` :!event `DamageTarget`))
  (set `self.DamageInfo` (make `/Game/DamageSystem/S_LX_DamageInfo` (/ _amount 2.0) _damagetype _damageresponse)))