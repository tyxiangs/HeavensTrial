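; BP_Enemy is a physics-driven enemy that can be grabbed and takes damage from sword slashes.
; Grabbing turns on heavily damped skeletal mesh physics, and release turns it off only while health remains.
; Slashes subtract health scaled by impulse magnitude, show it on a debug text render and play a slice sound, or at zero a kill sound with ragdoll and a blocking trace channel.
; Overlap events spawn blood particles at the impact point.
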(event `self.ReceiveBeginPlay`)

(event `/Game/BlueprintInterface/BPI_Interaction.InteractBegin`
  (params (Player :type "/Game/Blueprints/VRPawn Object Reference"))
  ; Grab
  (`PrimitiveComponent.SetSimulatePhysics` (`self.SkeletalMeshComponent`) true)
  (`PrimitiveComponent.SetLinearDamping` (`self.SkeletalMeshComponent`) 25.0))

(event `self.ReceiveHit`
  (params (MyComp :type "PrimitiveComponent Object Reference") (Other :type "Actor Object Reference") (OtherComp :type "PrimitiveComponent Object Reference") (bSelfMoved :type Boolean) (HitLocation :type "Vector Structure") (HitNormal :type "Vector Structure") (NormalImpulse :type "Vector Structure") (Hit :type "HitResult Structure (by ref)")))

(event `/Game/BlueprintInterface/BPI_Interaction.InteractEnd`
  (params (Player :type "/Game/Blueprints/VRPawn Object Reference"))
  ; Grab
  (if (> (`self.Health`) 0.0)
    (`PrimitiveComponent.SetSimulatePhysics` (`self.SkeletalMeshComponent`) false)
    (`PrimitiveComponent.SetLinearDamping` (`self.SkeletalMeshComponent`) 0.01)))

(event `self.ReceiveActorBeginOverlap`
  (params (OtherActor :type "Actor Object Reference")))

(event `/Game/BlueprintInterface/BPI_Slashable.Slash`
  (params (Impulse :type "Vector Structure"))
  (bind _returnvalue (`self.K2_GetActorLocation`))
  ; Calculate damage and update health
  (bind _output_get (set `self.Health` (- (`self.Health`) (/ (`KismetMathLibrary.VSize` Impulse) 1000.0))))
  ; Debug Info (Can delete)
  (`TextRenderComponent.K2_SetText` (`self.TextRender`) (`KismetTextLibrary.Conv_DoubleToText` _output_get "HalfToEven"))
  ; Check for death
  (if (<= _output_get 0.0)
    (`GameplayStatics.PlaySoundAtLocation` "/Game/Blueprints/Sword/kill.kill" _returnvalue (struct) 1.0 1.0 0.0 null null null null)
    (`PrimitiveComponent.SetSimulatePhysics` (`self.SkeletalMeshComponent`) true)
    (`PrimitiveComponent.SetCollisionResponseToChannel` (`self.SkeletalMeshComponent`) "ECC_GameTraceChannel1" "ECR_Block")
    (else
      (`GameplayStatics.PlaySoundAtLocation` "/Game/Blueprints/Sword/slice.slice" _returnvalue (struct) 1.0 1.0 0.0 null null null null))))

(event `/Game/BlueprintInterface/BPI_Overlappable.Overlap`
  (params (ImpactPoint :type "Vector Structure"))
  (`GameplayStatics.SpawnEmitterAtLocation` "/Game/Blueprints/Sword/P_Blood.P_Blood" ImpactPoint))

(fn `GetActor`
  (returns (Actor :type "Actor Object Reference"))
  (return null))

(fn `UserConstructionScript`)