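; BP_Sword is a sword actor that notifies actors it touches or cuts, passing hit point and slash velocity.
; Each tick it derives tip velocity from the tip's frame-to-frame movement, then traces from hilt root to tip on Visibility and sends OverlapMessage with the impact point to the hit actor.
; Mesh overlaps send SlashMessage with tip velocity relative to the overlapped component, so slashable actors must overlap the weapon.
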(event `self.ReceiveTick`
  (params (DeltaSeconds :type "Float (single-precision)"))
  (`self.SetSwordTipVelocity` DeltaSeconds)
  (bind (_outhit _returnvalue) (`KismetSystemLibrary.LineTraceSingle` (`SceneComponent.K2_GetComponentLocation` (`self.SwordRoot`)) (`SceneComponent.K2_GetComponentLocation` (`self.SwordTip`)) "TraceTypeQuery1"))
  (if _returnvalue
    (bind (_bblockinghit _binitialoverlap _time _distance _location _impactpoint _normal _impactnormal _physmat _hitactor) (`GameplayStatics.BreakHitResult` _outhit))
    (message `/Game/BlueprintInterface/BPI_Overlappable.Overlap` _hitactor _impactpoint)))

(event `self.SwordMesh.OnComponentBeginOverlap`
  (params (OverlappedComponent :type "PrimitiveComponent Object Reference") (OtherActor :type "Actor Object Reference") (OtherComp :type "PrimitiveComponent Object Reference") (OtherBodyIndex :type Integer) (bFromSweep :type Boolean) (SweepResult :type "HitResult Structure (by ref)"))
  ;[0.5 0.5 0.5 0.5] Calls Slash when sword overlaps. (Slashable actors should set collision with weapon as "Overlap")
  (message `/Game/BlueprintInterface/BPI_Slashable.Slash` OtherActor (- (`self.TipVelocity`) (`SceneComponent.GetComponentVelocity` OtherComp))))

(fn `SetSwordTipVelocity`
  (params (DeltaSeconds :type "Float (double-precision)"))
  (bind _returnvalue (`SceneComponent.K2_GetComponentLocation` (`self.SwordTip`)))
  (set `self.TipVelocity` (/ (- _returnvalue (`self.PreviousTipLocation`)) DeltaSeconds))
  (set `self.PreviousTipLocation` _returnvalue))

(fn `UserConstructionScript`)