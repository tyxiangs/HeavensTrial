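; BP_Scanner is a short-lived scanner actor in the WeakPoint folder, spawned with a VRPawn as owner.
; Each tick it adds ScanSpeed times delta time to its scale, clamping the vector length to a fixed magnitude.
; BeginPlay stores the owning VRPawn as Player and destroys the actor after a half-second delay, only if that cast succeeds.
; A Destroy event also removes it.
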(event `self.ReceiveTick`
  (params (DeltaSeconds :type "Float (single-precision)"))
  (`self.SetActorScale3D` (`KismetMathLibrary.ClampVectorSize` (+ (* DeltaSeconds (`self.Scan Speed`)) (`self.GetActorScale3D`)) 75.0 75.0)))

(event `self.ReceiveBeginPlay`
  (bind _asvrpawn (cast `/Game/Blueprints/VRPawn` (`self.GetOwner`)))
  (set `self.Player` _asvrpawn)
  (`KismetSystemLibrary.Delay` 0.5)
  (`self.K2_DestroyActor`))

(event `Destroy`
  (`self.K2_DestroyActor`))

(fn `UserConstructionScript`)