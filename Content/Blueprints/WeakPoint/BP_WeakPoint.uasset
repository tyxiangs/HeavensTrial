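; BP_WeakPoint is a weak point actor that blows up when activated and leaves a scanner in its place.
; Its Activate event plays an explosion sound and particle effect at the actor's location, spawns a BP_Scanner at the Sphere component's transform, then destroys the actor.
; Nothing in this graph calls Activate, and the overlap check against the player has no follow-up logic.
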(event `self.ReceiveActorBeginOverlap`
  (params (OtherActor :type "Actor Object Reference"))
  (if (== OtherActor (`self.Player`))
    _))

(event `Activate`
  (bind _returnvalue (`self.K2_GetActorLocation` self))
  (`GameplayStatics.SpawnSoundAtLocation` "/Game/StarterContent/Audio/Explosion_Cue.Explosion_Cue" _returnvalue (struct) 1.0 1.0 0.0 null null)
  (`GameplayStatics.SpawnEmitterAtLocation` "/Game/StarterContent/Particles/P_Explosion.P_Explosion" _returnvalue)
  (`|SpawnActorFromClass` "/Game/Blueprints/WeakPoint/BP_Scanner.BP_Scanner_C" (`SceneComponent.K2_GetComponentToWorld` (`self.Sphere`)) "Undefined" "MultiplyWithRoot" null null)
  (`self.K2_DestroyActor`))

(fn `UserConstructionScript`)