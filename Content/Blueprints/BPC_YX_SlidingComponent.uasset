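; Actor component that drives sliding movement for a VRPawn.
; Outside walking mode, Tick traces the ground and pushes the pawn forward at SlidingSpeed when slope angle and a normal-cross-up versus facing test pass.
; Otherwise Speed, applied through ChangeSpeed, decays each frame until sliding finishes; the direction test value is debug-printed.
; Slide is empty, and DashFunction and SlopeFunction are timer-based logic referenced only by each other and disconnected nodes.
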(event `self.ReceiveTick`
  (params (DeltaSeconds :type "Float (single-precision)"))
  (bind _player (`self.Player`))
  (bind _player_2 (`self.Player`))
  (bind _returnvalue (`Actor.K2_GetActorLocation` (`self.Player`)))
  (`|ExecutionSequence`
    (:`then_0`
      (if (`/Game/Blueprints/VRPawn.IsInWalkingMode` (`self.Player`))
        (if (`self.IsSlidingFinished`)
          (set `self.IsSliding` false)
          (set `self.IsStopTrigger` false)
          (elif (> (`self.Speed`) 5.0)
            (set `self.Speed` (- (`self.Speed`) (* DeltaSeconds 1000.0)))
            (else
              (set `self.IsSlidingFinished` true))))
        (else
          (set `self.IsSlidingFinished` false)
          (if (>= (`CharacterMovementComponent.MaxWalkSpeed` (`Character.CharacterMovement` (`self.Player`))) 0.0)
            (set `self.Speed` (- (`self.Speed`) (* DeltaSeconds 1000.0)))
            (`/Game/Blueprints/VRPawn.ChangeSpeed` (`self.Player`) (`self.Speed`))
            (bind _outhit (`KismetSystemLibrary.LineTraceSingle` _returnvalue (+ _returnvalue (0.0 0.0 -10000.0)) "TraceTypeQuery1"))
            (bind (_bblockinghit _binitialoverlap _time _distance _location _impactpoint _normal _impactnormal) (`GameplayStatics.BreakHitResult` _outhit))
            (bind _returnvalue_2 (`KismetMathLibrary.Dot_VectorVector` (`KismetMathLibrary.Cross_VectorVector` _impactnormal (0.0 0.0 1.0)) (`SceneComponent.GetForwardVector` (`Character.CapsuleComponent` (`self.Player`)))))
            (`KismetSystemLibrary.PrintString` (`KismetStringLibrary.Conv_DoubleToString` _returnvalue_2))
            (if (and (< _returnvalue_2 0.0) (> (`KismetMathLibrary.DegAcos` (`KismetMathLibrary.Dot_VectorVector` (0.0 0.0 1.0) _impactnormal)) 15.0))
              (set `self.IsSliding` true)
              (set `self.IsStopTrigger` false)
              (set `self.Speed` (`self.SlidingSpeed`))
              (`Pawn.AddMovementInput` _player (`SceneComponent.GetForwardVector` (`Character.CapsuleComponent` _player)) 1.0 false)
              (elif (not (`self.IsStopTrigger`))
                (set `self.Speed` (`self.Speed`))
                (`Pawn.AddMovementInput` _player_2 (`SceneComponent.GetForwardVector` (`Character.CapsuleComponent` _player_2)) 1.0 false)
                (if (`self.IsSliding`)
                  (set `self.IsSliding` false)
                  (elif (`self.IsStopTrigger`)
                    _
                    (elif (not (> (`self.Speed`) 0.0))
                      (set `self.IsStopTrigger` true)
                      (set `self.IsSlidingFinished` true))))))))))))

(event `self.ReceiveBeginPlay`
  (bind _asvrpawn (cast `/Game/Blueprints/VRPawn` (`self.GetOwner`)))
  (set `self.Player` _asvrpawn))

(event `Slide`)

(fn `DashFunction`
  (if (> (`self.Speed`) 50.0)
    (set `self.IsDashFinished` false)
    (else
      (`KismetSystemLibrary.K2_ClearTimer` null "DashFunction")
      (set `/Game/Blueprints/VRPawn.IsInWalkingMode` true (`self.Player`))
      (set `self.IsSlidingFinished` true)
      (set `self.IsDashFinished` true))))

(fn `SlopeFunction`
  (bind _player (`self.Player`))
  (bind _returnvalue (`Actor.K2_GetActorLocation` (`self.Player`)))
  (set `self.OnSlope` true)
  (bind _output_get (set `self.Speed` 3000.0))
  (`/Game/Blueprints/VRPawn.ChangeSpeed` (`self.Player`) _output_get)
  (`Pawn.AddMovementInput` _player (`SceneComponent.GetForwardVector` (`Character.CapsuleComponent` _player)) 1.0 false)
  (bind _outhit (`KismetSystemLibrary.LineTraceSingle` _returnvalue (+ _returnvalue (0.0 0.0 -10000.0)) "TraceTypeQuery1"))
  (if (> (`KismetMathLibrary.DegAcos` (`KismetMathLibrary.Dot_VectorVector` (0.0 0.0 1.0) (`.ImpactNormal` (`GameplayStatics.BreakHitResult` _outhit)))) 20.0)
    (`KismetSystemLibrary.K2_SetTimer` null "SlopeFunction" 0.0 true true)
    (else
      (set `self.OnSlope` false)
      (`self.DashFunction`))))